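; Player controller Blueprint that creates and manages the game HUD, escape menu and chat for non-dedicated-server instances.
; On BeginPlay it adds a GameHUD widget, passes it to MachHUD, and adds a hidden Menu widget.
; M or Escape toggles the menu along with cursor visibility and input ignoring, re-centering the mouse.
; Enter reveals and focuses the chat input, and OnClientMessage scrolls the chat log to the bottom.
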(event EventOnClientMessage
  (params (SenderPlayerState :type Player%20State%20Object%20Reference) (S :type String) (Type :type Name :default "None") (MsgLifeTime :type Float%20%28single-precision%29))
  (Class|ScrollBox|SetScrollOffset (Variables|/Game/UI/GameHUD.GameHUD_C|GetChatScroll (Utilities|Casting|CastToGameHUD (Variables|Default|GetGameHUDWidget))) 9999999999.0))

(event EventBeginPlay
  ;[1 1 1] Create widgets
  (if (not (Networking|IsDedicatedServer))
    (Utilities|FlowControl|Sequence
      (:then_0
        (bind _returnvalue (UserInterface|CreateWidget "/Game/UI/GameHUD.GameHUD_C" self))
        (Variables|Default|SetGameHUDWidget _returnvalue)
        (UserInterface|Viewport|AddtoViewport _returnvalue)
        (Variables|/Script/Mach.MachHUD|SetHUDWidget (Utilities|Casting|CastToMachHUD (HUD|GetHUD)) _returnvalue))
      (:then_1
        (bind _returnvalue_2 (UserInterface|CreateWidget "/Game/UI/Menu.Menu_C" self))
        (Variables|Default|SetEscapeMenuWidget _returnvalue_2)
        (UserInterface|Viewport|AddtoViewport _returnvalue_2)
        (Widget|SetVisibility _returnvalue_2 "Hidden")))))

(event Input|KeyboardEvents|Enter
  (bind _gamehudwidget (Variables|Default|GetGameHUDWidget))
  (bind _asgame_hud (Utilities|Casting|CastToGameHUD _gamehudwidget))
  (bind _chatinput (Variables|/Game/UI/GameHUD.GameHUD_C|GetChatInput _asgame_hud))
  (:Pressed
    (Widget|SetVisibility _chatinput "Visible")
    (Widget|SetKeyboardFocus _chatinput)))

(event Input|KeyboardEvents|M
  (bind (_sizex _sizey) (HUD|GetViewportSize))
  (bind _escapemenuwidget (Variables|Default|GetEscapeMenuWidget))
  ;[1 1 1] Toggle Escape Menu
  (:Pressed
    (Utilities|IsValid _escapemenuwidget
      (:Is%20Valid
        (if (not (Networking|IsDedicatedServer))
          (bind _returnvalue (Widget|GetVisibility _escapemenuwidget))
          (if (Utilities|Enum|Equal(Enum) _returnvalue "Hidden")
            (Widget|SetVisibility _escapemenuwidget "Visible")
            (else
              (Widget|SetVisibility _escapemenuwidget "Hidden")))
          (Variables|Default|SetbShowMouseCursor (Utilities|Enum|Equal(Enum) _returnvalue "Hidden"))
          (Class|MachPlayerController|SetIgnoreInput (Utilities|Enum|Equal(Enum) _returnvalue "Hidden"))
          (Class|MachPlayerController|SetMousePosition (/ _sizex 2) (/ _sizey 2)))))))

(event Input|KeyboardEvents|Escape
  (bind (_sizex _sizey) (HUD|GetViewportSize))
  (bind _escapemenuwidget (Variables|Default|GetEscapeMenuWidget))
  ;[1 1 1] Toggle Escape Menu
  (:Pressed
    (Utilities|IsValid _escapemenuwidget
      (:Is%20Valid
        (if (not (Networking|IsDedicatedServer))
          (bind _returnvalue (Widget|GetVisibility _escapemenuwidget))
          (if (Utilities|Enum|Equal(Enum) _returnvalue "Hidden")
            (Widget|SetVisibility _escapemenuwidget "Visible")
            (else
              (Widget|SetVisibility _escapemenuwidget "Hidden")))
          (Variables|Default|SetbShowMouseCursor (Utilities|Enum|Equal(Enum) _returnvalue "Hidden"))
          (Class|MachPlayerController|SetIgnoreInput (Utilities|Enum|Equal(Enum) _returnvalue "Hidden"))
          (Class|MachPlayerController|SetMousePosition (/ _sizex 2) (/ _sizey 2)))))))

(fn ConstructionScript)