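; Player character Blueprint that creates the game HUD and a menu widget on BeginPlay, with the menu starting hidden.
; M and Escape share one toggle that checks the menu's visibility to open or close it.
; Opening shows the cursor, centers it in the viewport and tells MachPlayerController to ignore input; closing hides the cursor and restores input.
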(event EventBeginPlay
  (bind _returnvalue (UserInterface|CreateWidget "/Game/UI/GameHUD.GameHUD_C"))
  (Variables|Default|SetGameHUDWidget _returnvalue)
  (UserInterface|Viewport|AddtoViewport (Variables|Default|GetGameHUDWidget))
  (bind _returnvalue_2 (UserInterface|CreateWidget "/Game/UI/Menu.Menu_C"))
  (Variables|Default|SetMenuWidget _returnvalue_2)
  (UserInterface|Viewport|AddtoViewport (Variables|Default|GetMenuWidget))
  (Widget|SetVisibility (Variables|Default|GetMenuWidget) "Hidden"))

(event Input|KeyboardEvents|Escape
  (bind _returnvalue (Game|GetPlayerController 0))
  (bind (_sizex _sizey) (HUD|GetViewportSize _returnvalue))
  (:Pressed
    (bind _returnvalue_2 (Widget|GetVisibility (Variables|Default|GetMenuWidget)))
    (if (Utilities|Enum|Equal(Enum) _returnvalue_2 "Hidden")
      (Widget|SetVisibility (Variables|Default|GetMenuWidget) "Visible")
      (Variables|/Script/Engine.PlayerController|SetbShowMouseCursor _returnvalue true)
      (bind _asmachplayercontroller (Utilities|Casting|CastToMachPlayerController _returnvalue))
      (Class|MachPlayerController|SetIgnoreInput _asmachplayercontroller true)
      (Class|MachPlayerController|SetMousePosition _asmachplayercontroller (/ _sizex 2) (/ _sizey 2))
      (else
        (Widget|SetVisibility (Variables|Default|GetMenuWidget) "Hidden")
        (Variables|/Script/Engine.PlayerController|SetbShowMouseCursor _returnvalue false)
        (bind _asmachplayercontroller_2 (Utilities|Casting|CastToMachPlayerController _returnvalue))
        (Class|MachPlayerController|SetIgnoreInput _asmachplayercontroller_2 false)))))

(event Input|KeyboardEvents|M
  (bind _returnvalue (Game|GetPlayerController 0))
  (bind (_sizex _sizey) (HUD|GetViewportSize _returnvalue))
  (:Pressed
    (bind _returnvalue_2 (Widget|GetVisibility (Variables|Default|GetMenuWidget)))
    (if (Utilities|Enum|Equal(Enum) _returnvalue_2 "Hidden")
      (Widget|SetVisibility (Variables|Default|GetMenuWidget) "Visible")
      (Variables|/Script/Engine.PlayerController|SetbShowMouseCursor _returnvalue true)
      (bind _asmachplayercontroller (Utilities|Casting|CastToMachPlayerController _returnvalue))
      (Class|MachPlayerController|SetIgnoreInput _asmachplayercontroller true)
      (Class|MachPlayerController|SetMousePosition _asmachplayercontroller (/ _sizex 2) (/ _sizey 2))
      (else
        (Widget|SetVisibility (Variables|Default|GetMenuWidget) "Hidden")
        (Variables|/Script/Engine.PlayerController|SetbShowMouseCursor _returnvalue false)
        (bind _asmachplayercontroller_2 (Utilities|Casting|CastToMachPlayerController _returnvalue))
        (Class|MachPlayerController|SetIgnoreInput _asmachplayercontroller_2 false)))))

(fn ConstructionScript)